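; BP_CylinderActor is a hit target for knives that makes a struck knife stop and spawns a replacement.
; On Hit, it casts its KnifeObject reference to Knife rather than using the hit actor, disables physics on that knife's N1Sasha component and clears its IsFluing flag.
; It then spawns a new Knife at the stored start transform.
; Hit and overlap events also print debug strings.
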(event EventBeginPlay)

(event Collision|EventActorBeginOverlap
  (params (OtherActor :type Actor%20Object%20Reference))
  (Development|PrintString "actor begin overlap"))

(event EventTick
  (params (DeltaSeconds :type Float%20%28single-precision%29)))

(event Collision|EventHit
  (params (MyComp :type Primitive%20Component%20Object%20Reference) (Other :type Actor%20Object%20Reference) (OtherComp :type Primitive%20Component%20Object%20Reference) (bSelfMoved :type Boolean) (HitLocation :type Vector :default "0, 0, 0") (HitNormal :type Vector :default "0, 0, 0") (NormalImpulse :type Vector :default "0, 0, 0") (Hit :type Hit%20Result%20Structure%20%28by%20ref%29))
  (Development|PrintString "Hit Cylinder")
  (bind _asknife (Utilities|Casting|CastToKnife (Variables|Default|GetKnifeObject)))
  (Physics|SetSimulatePhysics (Variables|/Game/Blueprints/Knife.Knife_C|GetN1Sasha _asknife) false)
  (Variables|/Game/Blueprints/Knife.Knife_C|SetisFluing _asknife false)
  (Game|SpawnActorfromClass "/Game/Blueprints/Knife.Knife_C" (Math|Transform|MakeTransform (Variables|/Game/Blueprints/Knife.Knife_C|GetStartPosition _asknife) (Variables|/Game/Blueprints/Knife.Knife_C|GetStartRotation _asknife) (Variables|/Game/Blueprints/Knife.Knife_C|GetStartScale _asknife)) "Undefined" 0 0))

(fn ConstructionScript)