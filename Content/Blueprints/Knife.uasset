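; Knife actor that glides into a target position and rotation, then launches when clicked.
; Each Tick, SmothMoveRotate interpolates the actor to its target transform until within tolerance, then marks it spawned.
; A click sets a flying flag; once spawned, Tick enables gravity on the N1Sasha component and applies an X impulse every frame.
; Overlap handling is empty, the knife respawn call is unwired, and the saved start transform is unused.
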(event EventBeginPlay
  (Variables|Default|SetStartPosition (Transformation|GetActorLocation))
  (Variables|Default|SetStartRotation (Transformation|GetActorRotation))
  (Variables|Default|SetStartScale (Transformation|GetActorScale3D)))

(event Collision|EventActorBeginOverlap
  (params (OtherActor :type Actor%20Object%20Reference)))

(event EventTick
  (params (DeltaSeconds :type Float%20%28single-precision%29))
  (CallFunction|SmothMoveRotate)
  (if (and (Variables|Default|GetisFluing) (Variables|Default|GetisSpawned))
    (Physics|SetEnableGravity (Variables|Default|GetN1Sasha) true)
    (Physics|AddImpulse (Variables|Default|GetN1Sasha) "30.000000, 0, 0" "None" false)))

(event MouseInput|EventActorOnClicked
  (params (ButtonPressed :type Key%20Structure :default "None"))
  (bind _output_get (Variables|Default|SetisToched true))
  (if _output_get
    (Variables|Default|SetisFluing true)))

(fn ConstructionScript)

(fn SmothMoveRotate
  (bind _returnvalue (Utilities|Time|GetWorldDeltaSeconds))
  (bind _targetrotation (Variables|Default|GetTargetRotation))
  (bind _n1sasha (Variables|Default|GetN1Sasha))
  (bind _targetposition (Variables|Default|GetTargetPosition))
  (bind _relativerotation (Variables|/Script/Engine.SceneComponent|GetRelativeRotation _n1sasha))
  (bind _relativelocation (Variables|/Script/Engine.SceneComponent|GetRelativeLocation _n1sasha))
  ;[1 1 1] Smooth move and rotation knife on spawn object
  (if (not (Variables|Default|GetisSpawned))
    (Transformation|SetActorLocation (Math|Interpolation|VInterpTo _relativelocation _targetposition _returnvalue 8.0) false false)
    (Transformation|SetActorRotation (Math|Interpolation|RInterpTo _relativerotation _targetrotation _returnvalue 8.0))
    (Variables|Default|SetisSpawned (and (Math|Vector|Equal(Vector) _relativelocation _targetposition 1.0) (Math|Rotator|Equal(Rotator) _relativerotation _targetrotation 1.0)))))